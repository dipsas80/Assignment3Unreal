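; BP_RagePickUp is a spinning potion pickup that grants rage to the player.
; When the player character overlaps it with rage below 100, it adds RageToAdd through Get/Set rage message calls and destroys itself, without clamping the total.
; Tick rotates the PotionBottle02 component around yaw at a frame-rate-independent speed.
; GetHealth is a stub that returns zero.
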(event EventBeginPlay)

(event Collision|EventActorBeginOverlap
  (params (OtherActor :type Actor%20Object%20Reference))
  (if (== OtherActor (Game|GetPlayerCharacter 0))
    (bind _value (Class|BIRageInterface|GetRage(Message) OtherActor))
    (if (< _value 1e+02)
      (Class|BIRageInterface|SetRage(Message) OtherActor (+ _value (Variables|Default|GetRageToAdd)))
      (Actor|DestroyActor))))

(event EventTick
  (params (DeltaSeconds :type Float%20%28single-precision%29))
  (Transformation|AddRelativeRotation (Variables|Default|Getpotion_bottle_02) (Math|Rotator|MakeRotator 0.0 0.0 (* DeltaSeconds 1e+02)) false false))

(fn ConstructionScript)

(fn GetHealth
  (return 0.0))