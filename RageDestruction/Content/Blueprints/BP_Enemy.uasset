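; Suicide-bomber enemy pawn that chases the player for a short time after sighting, then explodes on arrival, cutting player health and changing rage.
; Tick drives AIMoveTo while the follow timer runs and no stun is active, otherwise holding position and spinning once interest expires.
; GetHitData applies fixed damage through TakeDmg and returns a particle.
; Death plays gore effects, changes player rage and occasionally drops a pickup.
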(event OnSeePawn(PawnSensing)
  (params (Pawn :type Pawn%20Object%20Reference))
  ;[1 1 1] When see player
  (CallFunction|FollowDelayStart))

(event Custom|Take%20Dmg
  (params (damage :type Integer))
  ;[1 1 1] Take dmg event
  (Variables|Default|SetHealth (- (Variables|Default|GetHealth) damage))
  (if (<= (Variables|Default|GetHealth) 0.0)
    (Utilities|FlowControl|Sequence
      (:then_0
        (if (Math|Random|RandomBoolwithWeight 0.1)
          (Game|SpawnActorfromClass "/Game/Blueprints/BP_PickUp.BP_PickUp_C" (Transformation|GetActorTransform) "Undefined" 0 0)))
      (:then_1
        (Audio|PlaySound2D "/Game/Audio/splat.splat" 1.0 1.0 0.0 0 0)
        (Effects|SpawnEmitteratLocation "/Game/Realistic_Starter_VFX_Pack_Vol2/Particles/Blood/P_Blood_Splat_Cone.P_Blood_Splat_Cone" (Transformation|GetActorLocation))
        (Class|RageSteal|ChangeRage(Message) (Game|Player|GetPlayerPawn 0) 30)
        (Actor|DestroyActor)
        (Variables|Default|Setdead true)))))

(event Custom|Follow%20Delay%20Start
  ;[1 1 1] Start delay before it looses interest
  (Variables|Default|SetFollowDelay 5.0)
  (Variables|Default|SetHasSeen true))

(event EventTick
  (params (DeltaSeconds :type Float%20%28single-precision%29))
  (bind _returnvalue (Game|GetPlayerController 0))
  (bind _returnvalue_2 (Game|Player|GetPlayerPawn 0))
  ;[1 1 1] Move to player if not stunned or out of time
  (if (> (Variables|Default|GetFollowDelay) 0.0)
    (if (and (<= (Variables|Default|GetStunDelay) 0.0) (> (Variables|Default|GetFollowDelay) 0.0))
      (AI|AIMoveTo self (Transformation|GetActorLocation _returnvalue) _returnvalue 2e+02 false
        (:then
          (Variables|Default|SetFollowDelay (- (Variables|Default|GetFollowDelay) DeltaSeconds) :!label _label)
          (Variables|Default|SetStunDelay (- (Variables|Default|GetStunDelay) DeltaSeconds)))
        (:OnSuccess
          (Effects|SpawnEmitteratLocation "/Game/StarterContent/Particles/P_Explosion.P_Explosion" (Transformation|GetActorLocation))
          (if (not (Variables|Default|Getdead))
            (Class|RageSteal|ChangeRage(Message) _returnvalue_2 10)
            (bind _health (Class|BIHealthInterface|GetHealth(Message) _returnvalue_2))
            (Class|BIHealthInterface|SetHealth(Message) _returnvalue_2 (- _health 1e+01))
            (Audio|PlaySound2D "/Game/StarterContent/Audio/Explosion02.Explosion02" 1.0 1.0 0.0 0 0)
            (Actor|DestroyActor))))
      (else
        (goto _label)))
    (else
      (AI|AIMoveTo self (Transformation|GetActorLocation) 0 5.0 false
        (:then
          (Transformation|AddActorLocalRotation "0,2.000000, 0" false false))))))

(event EventBeginPlay
  ;[1 1 1] Setup
  (Pawn|SpawnDefaultController))

(fn ConstructionScript)

(fn GetHitData
  (CallFunction|TakeDmg self 34)
  (return (Variables|Default|Getparticle)))

(fn RageGather
  (return 0))