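; Enemy AI actor that chases and attacks the player on sight via PawnSensing and AI MoveTo.
; Attacks resolve when a timeline ends, draining player health and adding rage if still in range.
; GetHitData applies fixed damage and returns a particle; damage halts movement and briefly stuns, blocking chase.
; Death grants the player rage, then after a delay spawns a BP_PickUp and destroys the enemy.
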(event OnSeePawn(PawnSensing)
  (params (Pawn :type Pawn%20Object%20Reference))
  ;[1 1 1] When seeing player
  (Variables|Default|SetisSeeingPlayer true)
  (if (<= (Math|Vector|Distance(Vector) (Transformation|GetActorLocation (Game|GetPlayerCharacter 0)) (Transformation|GetActorLocation self)) 2e+02)
    (CallFunction|Attack)
    (else
      (CallFunction|FollowPlayer))))

(event Custom|FollowPlayer
  (bind _returnvalue (Game|GetPlayerCharacter 0))
  ;[1 1 1] Follow Player if seen
  (if (Variables|Default|GetisSeeingPlayer)
    (if (Utilities|IsValid _returnvalue)
      (if (not (Variables|Default|Getstunned))
        (AI|AIMoveTo self "0, 0, 0" _returnvalue 5.0 false)))))

(event Custom|Killed
  ;[1 1 1] Kill Logic
  (if (not (Variables|Default|Getdead))
    (Class|RageSteal|ChangeRage(Message) (Game|GetPlayerCharacter 0) (Variables|Default|GetRageValue))
    (Variables|Default|Setdead true)
    (Utilities|FlowControl|Delay 0.6)
    (Game|SpawnActorfromClass "/Game/Blueprints/BP_PickUp.BP_PickUp_C" (Transformation|GetActorTransform self) "Undefined" 0 0)
    (Actor|DestroyActor self)))

(event Custom|TakeDmg
  (params (dmg :type Integer))
  ;[1 1 1] Dmg Calc
  (Variables|Default|SetHasSeen true)
  (Variables|Default|SetHealth (- (Variables|Default|GetHealth) dmg))
  (CallFunction|StunCD 1.0)
  (AI|AIMoveTo self (Transformation|GetActorLocation) 0 5.0 false
    (:then
      (if (<= (Variables|Default|GetHealth) 0.0)
        (CallFunction|Killed)))))

(event Custom|StunCD
  (params (StunTime :type Float%20%28double-precision%29))
  (Variables|Default|Setstunned true)
  (Timeline|Stun Play
    (:Finished
      (Variables|Default|Setstunned false))))

(event Custom|Attack
  (bind _returnvalue (Game|GetPlayerCharacter 0))
  (Timeline|AttackDuration Play
    (:Finished
      (if (<= (Math|Vector|Distance(Vector) (Transformation|GetActorLocation (Game|GetPlayerCharacter 0)) (Transformation|GetActorLocation self)) 2e+02)
        (bind _health (Class|BIHealthInterface|GetHealth(Message) _returnvalue))
        (Class|BIHealthInterface|SetHealth(Message) _returnvalue (- _health 1e+01))
        (Class|RageSteal|ChangeRage(Message) _returnvalue 10)))))

(event EventBeginPlay
  (Pawn|SpawnDefaultController))

(event Collision|EventActorBeginOverlap
  (params (OtherActor :type Actor%20Object%20Reference)))

(fn ConstructionScript)

(fn GetHitData
  (CallFunction|TakeDmg self 25)
  (return (Variables|Default|Getparticle)))

(fn RageGather
  (return 0))